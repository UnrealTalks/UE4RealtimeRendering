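; Procedural staircase with glass balustrades, built in the construction script from a step count and tread dimensions, with no runtime logic.
; Treads are mesh instances at a fixed rise, spaced slightly closer than their depth.
; Each step gets a procedural glass quad on both sides, with identical winding and normals.
; A second instanced mesh supplies lower beams and upper rails, stretched and rotated along the slope.
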(fn `Make Glass Wall`
  (params (TreadLocation :type "Vector Structure") (NextTreadLocation :type "Vector Structure"))
  (bind _returnvalue (/ (- NextTreadLocation TreadLocation) 2.2))
  (bind _returnvalue_2 (/ (- TreadLocation NextTreadLocation) 2.2))
  (bind _returnvalue_3 (+ _returnvalue (0.0 0.0 92.0)))
  (bind _returnvalue_4 (`AddComponent|NODE_AddProceduralMeshComponent-0` :`RelativeTransform` (`KismetMathLibrary.MakeTransform` TreadLocation (struct) (1.0 1.0 1.0))))
  (`ProceduralMeshComponent.CreateMeshSection_LinearColor` :`self` _returnvalue_4 :`Vertices` (`|MakeArray` _returnvalue_2 (+ _returnvalue_2 (0.0 0.0 92.0)) _returnvalue_3 _returnvalue_3 _returnvalue _returnvalue_2) :`Triangles` (`|MakeArray` 0 1 2 3 4 5) :`Normals` (`|MakeArray` (0.0 -1.0 0.0) (0.0 -1.0 0.0) (0.0 -1.0 0.0) (0.0 -1.0 0.0) (0.0 -1.0 0.0) (0.0 -1.0 0.0) :!type "Vector Structure"))
  (`PrimitiveComponent.SetMaterial` _returnvalue_4 0 "/Game/Materials/M_Glass.M_Glass"))

(fn `UserConstructionScript`
  (bind _treaddimensions (`self.TreadDimensions`))
  (bind _instancedstaticmesh1 (`self.InstancedStaticMesh1`))
  (bind _numberofsteps (`self.NumberOfSteps`))
  (bind (_treaddimensions_x _treaddimensions_y) (`KismetMathLibrary.BreakVector` (`self.TreadDimensions`)))
  (bind _instancedstaticmesh1_2 (`self.InstancedStaticMesh1`))
  (bind _y (.y (`self.TreadDimensions`)))
  (bind _y_2 (.y (`self.TreadDimensions`)))
  (bind _returnvalue (* (.x _treaddimensions) 0.8))
  (bind _returnvalue_2 (* (+ _numberofsteps 4) _returnvalue))
  (bind _returnvalue_3 (`KismetMathLibrary.MakeVector` 0.0 (/ _y_2 2.0)))
  (bind _returnvalue_4 (`KismetMathLibrary.MakeVector` 0.0 (/ _y_2 -2.0)))
  (bind _returnvalue_5 (`KismetMathLibrary.MakeVector` (/ (* _numberofsteps _returnvalue) 2.0) 0.0 (/ (* _numberofsteps 20.0) 2.0)))
  (bind _returnvalue_6 (`KismetMathLibrary.Conv_VectorToRotator` _returnvalue_5))
  (for _index (range (+ (`self.NumberOfSteps`) 1))
    (bind _returnvalue_7 (* _index _returnvalue))
    (bind _returnvalue_8 (* _index 20.0))
    (`InstancedStaticMeshComponent.AddInstance` (`self.InstancedStaticMesh`) (`KismetMathLibrary.MakeTransform` (`KismetMathLibrary.MakeVector` _returnvalue_7 0.0 _returnvalue_8) (struct) _treaddimensions))
    (bind _returnvalue_9 (`KismetMathLibrary.MakeVector` _returnvalue_7 0.0 _returnvalue_8))
    (bind _returnvalue_10 (+ _index 1))
    (bind _returnvalue_11 (`KismetMathLibrary.MakeVector` (* _returnvalue_10 _returnvalue) 0.0 (* _returnvalue_10 20.0)))
    (`self.Make Glass Wall` (+ _returnvalue_3 _returnvalue_9) (+ _returnvalue_3 _returnvalue_11))
    (`self.Make Glass Wall` (+ _returnvalue_4 _returnvalue_9) (+ _returnvalue_4 _returnvalue_11)))
  (`InstancedStaticMeshComponent.AddInstance` _instancedstaticmesh1_2 (`KismetMathLibrary.MakeTransform` (+ (`KismetMathLibrary.MakeVector` 0.0 (/ _treaddimensions_y -2.0)) _returnvalue_5) _returnvalue_6 (`KismetMathLibrary.MakeVector` _returnvalue_2 10.0 30.0)))
  (`InstancedStaticMeshComponent.AddInstance` _instancedstaticmesh1_2 (`KismetMathLibrary.MakeTransform` (+ (`KismetMathLibrary.MakeVector` 0.0 (/ _treaddimensions_y 2.0)) _returnvalue_5) _returnvalue_6 (`KismetMathLibrary.MakeVector` _returnvalue_2 10.0 30.0)))
  (`InstancedStaticMeshComponent.AddInstance` _instancedstaticmesh1 (`KismetMathLibrary.MakeTransform` (+ _returnvalue_5 (`KismetMathLibrary.MakeVector` 0.0 (/ _y 2.0) 92.0)) _returnvalue_6 (`KismetMathLibrary.MakeVector` _returnvalue_2 10.0 5.0)))
  (`InstancedStaticMeshComponent.AddInstance` _instancedstaticmesh1 (`KismetMathLibrary.MakeTransform` (+ _returnvalue_5 (`KismetMathLibrary.MakeVector` 0.0 (/ _y -2.0) 92.0)) _returnvalue_6 (`KismetMathLibrary.MakeVector` _returnvalue_2 10.0 5.0))))