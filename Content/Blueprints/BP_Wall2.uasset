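; BP_Wall2 is a procedural wall with a grid of windows, built entirely in the Construction Script from dimension and count variables.
; Stretched static mesh components form vertical and horizontal strips between the windows, sized from the wall space the windows leave.
; MakeWindow adds four frame pieces per cell and calls NewFunction0 for the dividing bars on each axis.
; When Lights is set, each window also gets a window-sized rect light.
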(fn `MakeWindow`
  (params (XOffset :type "Float (double-precision)") (ZOffset :type "Float (double-precision)"))
  (bind _xoffset (`local.XOffset`))
  (bind _zoffset (`local.ZOffset`))
  (bind _framedepth (`self.FrameDepth`))
  (bind _framethickness (`self.FrameThickness`))
  (bind (_totalwalldimensions_x _totalwalldimensions_y) (`KismetMathLibrary.BreakVector` (`self.TotalWallDimensions`)))
  (bind _windowwidth (`self.WindowWidth`))
  (bind _windowheight (`self.WindowHeight`))
  (bind _returnvalue (/ (`self.WindowHeight`) 2.0))
  (bind _returnvalue_2 (/ (`self.WindowWidth`) 2.0))
  (`AddComponent|NODE_AddStaticMeshComponent-8` :`RelativeTransform` (`KismetMathLibrary.MakeTransform` (`KismetMathLibrary.MakeVector` XOffset 0.0 (+ ZOffset _returnvalue)) (struct) (`KismetMathLibrary.MakeVector` _windowwidth _framedepth _framethickness)))
  (`AddComponent|NODE_AddStaticMeshComponent-9` :`RelativeTransform` (`KismetMathLibrary.MakeTransform` (`KismetMathLibrary.MakeVector` XOffset 0.0 (+ ZOffset (* _returnvalue -1.0))) (struct) (`KismetMathLibrary.MakeVector` _windowwidth _framedepth _framethickness)))
  (`AddComponent|NODE_AddStaticMeshComponent-10` :`RelativeTransform` (`KismetMathLibrary.MakeTransform` (`KismetMathLibrary.MakeVector` (+ XOffset _returnvalue_2) 0.0 ZOffset) (struct) (`KismetMathLibrary.MakeVector` _framethickness _framedepth _windowheight)))
  (`AddComponent|NODE_AddStaticMeshComponent-11` :`RelativeTransform` (`KismetMathLibrary.MakeTransform` (`KismetMathLibrary.MakeVector` (+ XOffset (* _returnvalue_2 -1.0)) 0.0 ZOffset) (struct) (`KismetMathLibrary.MakeVector` _framethickness _framedepth _windowheight)))
  (`self.NewFunction_0` (`self.DivisionsX`) (`self.WindowHeight`) (`self.WindowWidth`) true _xoffset _zoffset)
  (`self.NewFunction_0` (`self.DivisionsY`) (`self.WindowWidth`) (`self.WindowHeight`) false _xoffset _zoffset)
  (if (`self.Lights?`)
    (bind _returnvalue_3 (`AddComponent|NODE_AddRectLightComponent-0` :`RelativeTransform` (`KismetMathLibrary.MakeTransform` (`KismetMathLibrary.MakeVector` (`local.XOffset`) _totalwalldimensions_y (`local.ZOffset`)) (struct :`Yaw` 90.0))))
    (`RectLightComponent.SetSourceWidth` _returnvalue_3 (`self.WindowWidth`))
    (`RectLightComponent.SetSourceHeight` _returnvalue_3 (`self.WindowHeight`))
    (`LocalLightComponent.SetAttenuationRadius` _returnvalue_3 (`self.LightRadius`))
    (`LightComponent.SetIntensity` _returnvalue_3 (`self.Intensity`))))

(fn `NewFunction_0`
  (params (Divisions :type Integer) (`Pane Length` :type "Float (double-precision)") (`Pane Span` :type "Float (double-precision)") (XDir :type Boolean) (XOffset :type "Float (double-precision)") (YOffset :type "Float (double-precision)"))
  (bind _panethickness (`self.PaneThickness`))
  (for _index (range 1 Divisions)
    (if XDir
      (bind _returnvalue (- (* _index (/ `Pane Span` (`KismetMathLibrary.Conv_IntToDouble` Divisions))) (/ `Pane Span` 2.0)))
      (`AddComponent|NODE_AddStaticMeshComponent-6` :`RelativeTransform` (`KismetMathLibrary.MakeTransform` (`KismetMathLibrary.MakeVector` (+ (`local.XOffset`) _returnvalue) 0.0 (`local.YOffset`)) (struct) (`KismetMathLibrary.MakeVector` _panethickness _panethickness (`local.Pane Length`))))
      (else
        (`AddComponent|NODE_AddStaticMeshComponent-7` :`RelativeTransform` (`KismetMathLibrary.MakeTransform` (`KismetMathLibrary.MakeVector` (`local.XOffset`) 0.0 (+ _returnvalue (`local.YOffset`))) (struct) (`KismetMathLibrary.MakeVector` (`local.Pane Length`) _panethickness _panethickness)))))))

(fn `UserConstructionScript`
  (bind (_totalwalldimensions_x _totalwalldimensions_y _totalwalldimensions_z) (`KismetMathLibrary.BreakVector` (`self.TotalWallDimensions`)))
  (bind (_totalwalldimensions_x_2 _totalwalldimensions_y_2 _totalwalldimensions_z_2) (`KismetMathLibrary.BreakVector` (`self.TotalWallDimensions`)))
  (bind _totalwalldimensions_x_3 (`KismetMathLibrary.BreakVector` (`self.TotalWallDimensions`)))
  (bind _numberofwindowsx (`self.NumberOfWindowsX`))
  (bind _numberofwindowsz (`self.NumberOfWindowsZ`))
  (bind (_totalwalldimensions_x_4 _totalwalldimensions_y_3 _totalwalldimensions_z_3) (`KismetMathLibrary.BreakVector` (`self.TotalWallDimensions`)))
  (bind (_totalwalldimensions_x_5 _totalwalldimensions_y_4 _totalwalldimensions_z_4) (`KismetMathLibrary.BreakVector` (`self.TotalWallDimensions`)))
  (bind _numberofwindowsx_2 (`self.NumberOfWindowsX`))
  (bind _totalwalldimensions_x_6 (`KismetMathLibrary.BreakVector` (`self.TotalWallDimensions`)))
  (bind _numberofwindowsz_2 (`self.NumberOfWindowsZ`))
  (bind _returnvalue (`KismetMathLibrary.Conv_IntToDouble` _numberofwindowsz_2))
  (bind _returnvalue_2 (/ (- _totalwalldimensions_x_6 (`KismetMathLibrary.Conv_IntToDouble` _numberofwindowsx_2)) (`KismetMathLibrary.Conv_IntToDouble` _numberofwindowsx_2)))
  (bind _returnvalue_3 (/ (- _totalwalldimensions_z_4 _returnvalue) _returnvalue))
  (for _index (range _numberofwindowsx_2)
    (for _index_2 (range _numberofwindowsz_2)
      (`self.MakeWindow` (+ (* _index _returnvalue_2) (/ _returnvalue_2 2.0)) (+ (* _index_2 _returnvalue_3) (/ _returnvalue_3 2.0)))))
  (for _index_3 (range (+ _numberofwindowsx 1))
    (`AddComponent|NODE_AddStaticMeshComponent-12` :`RelativeTransform` (`KismetMathLibrary.MakeTransform` (`KismetMathLibrary.MakeVector` (* _index_3 (/ (- _totalwalldimensions_x_3 (`KismetMathLibrary.Conv_IntToDouble` _numberofwindowsx)) (`KismetMathLibrary.Conv_IntToDouble` _numberofwindowsx))) 0.0 (/ _totalwalldimensions_z_2 2.0)) (struct) (`KismetMathLibrary.MakeVector` (/ (- _totalwalldimensions_x_3 (* _numberofwindowsx (`self.WindowWidth`))) (`KismetMathLibrary.Conv_IntToDouble` _numberofwindowsx)) _totalwalldimensions_y_2 _totalwalldimensions_z_2))))
  (for _index_4 (range (+ _numberofwindowsz 1))
    (`AddComponent|NODE_AddStaticMeshComponent-13` :`RelativeTransform` (`KismetMathLibrary.MakeTransform` (`KismetMathLibrary.MakeVector` (/ _totalwalldimensions_x_4 2.0) 0.0 (* _index_4 (/ (- _totalwalldimensions_z_3 (`KismetMathLibrary.Conv_IntToDouble` _numberofwindowsz)) (`KismetMathLibrary.Conv_IntToDouble` _numberofwindowsz)))) (struct) (`KismetMathLibrary.MakeVector` _totalwalldimensions_x _totalwalldimensions_y (/ (- _totalwalldimensions_z_3 (* _numberofwindowsz (`self.WindowHeight`))) (`KismetMathLibrary.Conv_IntToDouble` _numberofwindowsz)))))))